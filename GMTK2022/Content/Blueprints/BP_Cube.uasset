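; BP_Cube is an actor that pairs a steadily pitching Cube with a perpetually bouncing physics Sphere.
; Each Tick spins the Cube, boosts the Sphere upward when its vertical velocity is near zero, then clamps that velocity while preserving horizontal motion.
; Sphere hits play a thud at the impact point and add a random upward velocity, keeping the bounce going.
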(event OnComponentHit(Sphere)
  (params (HitComponent :type Primitive%20Component%20Object%20Reference) (OtherActor :type Actor%20Object%20Reference) (OtherComp :type Primitive%20Component%20Object%20Reference) (NormalImpulse :type Vector :default "0, 0, 0") (Hit :type Hit%20Result%20Structure%20%28by%20ref%29))
  (Audio|PlaySoundatLocation "/Game/SFX/Effects/Thud.Thud" (.ImpactPoint (Collision|BreakHitResult Hit)) "0, 0, 0" 1.0 1.0 0.0 0 0 0)
  (Physics|SetPhysicsLinearVelocity (Variables|Default|GetSphere) (Math|Vector|MakeVector 0.0 0.0 (Math|Random|RandomFloatinRange 6e+02 8e+02)) true "None"))

(event EventTick
  (params (DeltaSeconds :type Float%20%28single-precision%29))
  (bind _sphere (Variables|Default|GetSphere))
  (Transformation|AddWorldRotation (Variables|Default|GetCube) (Math|Rotator|MakeRotator 0.0 (* DeltaSeconds -1e+02) 0.0) false false)
  (bind _returnvalue (Physics|GetPhysicsLinearVelocity (Variables|Default|GetSphere) "None"))
  (if (Math|Float|NearlyEqual(Float) (.z _returnvalue) 0.0 0.1)
    (Physics|SetPhysicsLinearVelocity (Variables|Default|GetSphere) (Math|Vector|MakeVector 0.0 0.0 6e+02) true "None"))
  (bind _returnvalue_2 (Physics|GetPhysicsLinearVelocity _sphere "None"))
  (Physics|SetPhysicsLinearVelocity _sphere (Math|Vector|MakeVector (.x _returnvalue_2) (.y _returnvalue_2) (Math|Float|Clamp(Float) (.z _returnvalue_2) -1e+03 7e+02)) false "None"))

(fn ConstructionScript)