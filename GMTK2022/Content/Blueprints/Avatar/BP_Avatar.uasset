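; BP_Avatar is the player character: once started, it auto-runs forward while tethered to a held sphere by a physics constraint.
; Scroll input adjusts walk speed against a per-tick decay.
; Exceeding Fallzone eases speed down and triggers a randomly repeating roll, blending spine-down physical animation until a timeline restores control.
; It also starts persistent menu music with a timed switch, and opens a pause menu that mutes it.
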(event Custom|Recovered
  (bind _mesh (Variables|Character|GetMesh))
  (Utilities|FlowControl|DoOnce false) ; enters at Reset
)

(event Custom|Tick2
  (bind _charactermovement (Variables|Character|GetCharacterMovement))
  (Variables|/Script/Engine.CharacterMovementComponent|SetMaxWalkSpeed _charactermovement (- (Class|MovementComponent|GetMaxSpeed _charactermovement) (Variables|Default|GetScrollPointNeededSpeed))))

(event EventTick
  (params (DeltaSeconds :type Float%20%28single-precision%29))
  (bind _mesh (Variables|Character|GetMesh))
  (Utilities|FlowControl|Gate true
    (:Exit
      (CallFunction|Tick2)
      (Pawn|Input|AddMovementInput (Transformation|GetActorForwardVector self) 1.0 true)
      (Variables|Default|SetScrollPointNeeded (+ (Variables|Default|GetScrollPointNeeded) (* 1.0 (Variables|Default|GetScrollPointNeededSpeed))))
      (if (> (Class|MovementComponent|GetMaxSpeed (Variables|Character|GetCharacterMovement)) (Variables|Default|GetFallzone))
        (Variables|/Script/Engine.CharacterMovementComponent|SetMaxWalkSpeed (Variables|Character|GetCharacterMovement) (Math|Interpolation|FInterpTo (Class|MovementComponent|GetMaxSpeed (Variables|Character|GetCharacterMovement)) 5e+02 (Utilities|Time|GetWorldDeltaSeconds) 4.0))
        (Utilities|FlowControl|DoOnce false
          (:Completed
            (Variables|Default|SetRunOngoing false)
            (Animation|Montage|PlayMontage _mesh "/Game/Anims/Roll_Montage.Roll_Montage"
              (:then
                (Class|SkeletalMeshComponent|SetAllBodiesBelowSimulatePhysics _mesh (Utilities|Name|MakeLiteralName "Spine") true true)
                (Class|PhysicalAnimationComponent|ApplyPhysicalAnimationProfileBelow (Variables|Default|GetPhysicalAnimation) "Spine" "InControl" false false)
                (Class|SkeletalMeshComponent|SetAllBodiesBelowPhysicsBlendWeight (Variables|Character|GetMesh) (Utilities|Name|MakeLiteralName "Spine") 0.4 false true))
              (:OnCompleted
                (Animation|Montage|PlayMontage _mesh "/Game/Anims/Roll_Montage.Roll_Montage" :!label _label
                  (:OnBlendOut
                    (if (Math|Random|RandomBool)
                      (goto _label)
                      (else
                        (bind _speed (Timeline|Speed PlayFromStart)
                          (:Update
                            (Class|SkeletalMeshComponent|SetAllBodiesBelowPhysicsBlendWeight (Variables|Character|GetMesh) (Utilities|Name|MakeLiteralName "Spine") _speed false true))
                          (:Finished
                            (Class|SkeletalMeshComponent|SetAllBodiesBelowSimulatePhysics (Variables|Character|GetMesh) (Utilities|Name|MakeLiteralName "Spine") false true)
                            (Variables|Default|SetScrollPointNeeded 0.0)
                            (Variables|Default|SetScrollPoint 0.0)
                            (Variables|Default|SetRunOngoing true)
                            (CallFunction|Recovered)))))))))))
        (else
          (Development|PrintString (Utilities|String|ToString(Float) 0.0) true true "(R=0.000000,G=0.660000,B=1.000000,A=1.000000)" 0.0))))))

(event EventBeginPlay
  (Utilities|FlowControl|Sequence
    (:then_0
      (Class|PhysicalAnimationComponent|SetSkeletalMeshComponent (Variables|Default|GetPhysicalAnimation) (Variables|Character|GetMesh)))
    (:then_1
      (bind _returnvalue (Audio|CreateSound2D (Variables|Default|GetMenuMusic) 1.0 1.0 0.0 0 true))
      (Variables|Default|SetLevelMusic _returnvalue)
      (Audio|Components|Audio|Play _returnvalue 0.0)
      (Utilities|FlowControl|Delay 22.588232)
      (Effects|Components|ParticleSystem|SetBoolParameter _returnvalue "switch" true))))

(event Input|ActionEvents|InputActionStartGame
  (params (Key :type Key%20Structure :default "None"))
  (bind _mesh (Variables|Character|GetMesh))
  (:Pressed
    (Variables|Default|SetRunOngoing true)
    (Variables|/Game/Anims/ABP_Avatar.ABP_Avatar_C|SetRunning (.AsABP%20Avatar (Utilities|Casting|CastToABP_Avatar (Components|SkeletalMesh|GetAnimInstance (Variables|Character|GetMesh)))) true)
    (CallFunction|Grab)
    (Utilities|FlowControl|Gate true) ; enters at Open
  ))

(event Input|ActionEvents|InputActionPause
  (params (Key :type Key%20Structure :default "None"))
  (bind _returnvalue (Game|GetPlayerController 0))
  (:Pressed
    (Audio|Components|Audio|SetVolumeMultiplier (Variables|Default|GetLevelMusic) 0.0 :!class /Script/Engine.AudioComponent)
    (Game|SetGamePaused true)
    (bind _returnvalue_2 (UserInterface|CreateWidget "/Game/UI/Pause.Pause_C"))
    (UserInterface|Viewport|AddtoViewport _returnvalue_2 0)
    (Input|SetInputModeUIOnly _returnvalue _returnvalue_2 "DoNotLock")
    (Variables|/Script/Engine.PlayerController|SetbShowMouseCursor _returnvalue true)))

(event Input|AxisEvents|InputAxisScroll
  (params (AxisValue :type Float%20%28single-precision%29))
  (bind _charactermovement (Variables|Character|GetCharacterMovement))
  (if (Variables|Default|GetRunOngoing)
    (bind _output_get (Variables|Default|SetScrollPoint (+ (* AxisValue (Variables|Default|GetScrollPointSpeed)) (Variables|Default|GetScrollPoint))))
    (Variables|/Script/Engine.CharacterMovementComponent|SetMaxWalkSpeed _charactermovement (Math|Float|Clamp(Float) (+ _output_get (Class|MovementComponent|GetMaxSpeed _charactermovement)) 4e+02 4e+03))))

(fn ConstructionScript)

(fn Grab
  (bind _cuberef (Variables|Default|GetCubeRef))
  (bind _sphere (Variables|/Game/Blueprints/BP_Cube.BP_Cube_C|GetSphere _cuberef))
  (Transformation|SetRelativeLocation (Variables|Default|GetHeldObjectSlot) "1500.000000, 0, 0" false false)
  (Class|PhysicsConstraintComponent|SetConstrainedComponents (Variables|Default|GetGrabConstraint) (Variables|Default|GetHeldObjectSlot) "None" _sphere "None")
  (Collision|SetCollisionResponsetoChannel _sphere "ECC_Pawn" "ECR_Ignore"))

(fn ScrollDifference
  (return (- (Variables|Default|GetScrollPointNeeded) (Variables|Default|GetScrollPoint))))